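; BP_Item is a physics-simulated world item that the player can highlight and add to a backpack.
; On BeginPlay it caches the mesh's first material as ItemTexture and enables physics.
; Hover events toggle an outline through the mesh's overlay material, and EquipItem passes the item to the player via an AddItemToBackpack message.
; GetHealth and UpdateInventory are empty stubs.
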(event EventBeginPlay
  (Variables|Default|SetItemTexture (Rendering|Material|GetMaterial (Variables|Default|GetItemMesh) 0))
  (Physics|SetSimulatePhysics (Variables|Default|GetItemMesh) true))

(event Collision|EventActorBeginOverlap
  (params (OtherActor :type Actor%20Object%20Reference)))

(event EventTick
  (params (DeltaSeconds :type Float%20%28single-precision%29)))

(event EventEquipItem
  (params (Player :type Actor%20Object%20Reference))
  (Class|BIItem|AddItemtoBackpack(Message) Player self))

(event EventStartHover
  (Rendering|Material|SetOverlayMaterial (Variables|Default|GetItemMesh) "/Game/Materials/M_InteractionOutline.M_InteractionOutline" :!class /Script/Engine.MeshComponent))

(event EventEndHover
  (Rendering|Material|SetOverlayMaterial (Variables|Default|GetItemMesh) 0 :!class /Script/Engine.MeshComponent))

(fn ConstructionScript)

(fn GetHealth
  (return 0.0 0.0))

(fn UpdateInventory
  (params (ItemList :type Array%20of%20BP%20Item%20Class%20References))
  (return))